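; BP_Thunder is a player lightning strike actor that damages overlapping actors tagged Dragon by its ThunderDamage amount.
; On BeginPlay it stores its spawn location and feeds it to the three beam start and end pairs of a Niagara spark effect.
; The beams run vertically, ending at the actor's position and starting at the same XY with Z left unset, and a 2D thunder sound plays.
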(event `self.ReceiveTick`
  (params (DeltaSeconds :type "Float (single-precision)")))

(event `self.ReceiveActorBeginOverlap`
  (params (OtherActor :type "Actor Object Reference"))
  ;[1 1 1] 当たったときにダメージを与える
  (if (`self.ActorHasTag` OtherActor (`self.Dragon`))
    (`GameplayStatics.ApplyDamage` OtherActor (`self.Thunder_Damage`))))

(event `self.ReceiveBeginPlay`
  (bind (_returnvalue_x _returnvalue_y _returnvalue_z) (`KismetMathLibrary.BreakVector` (`self.K2_GetActorLocation`)))
  (`|ExecutionSequence`
    (:`then_0`
      ;[1 1 1] Start地点とEnd地点のXとYの座標を決める
      (set `self.Spawn_Location_X` _returnvalue_x)
      (set `self.Spawn_Location_Y` _returnvalue_y)
      (set `self.Spawn_Location_Z` _returnvalue_z))
    (:`then_1`
      ;[1 1 1] 雷のエフェクトの座標指定
      (`NiagaraComponent.SetVariableVec3` (`self.Nia_Spark001_00`) "Beam End01" (`KismetMathLibrary.MakeVector` (`self.Spawn_Location_X`) (`self.Spawn_Location_Y`) (`self.Spawn_Location_Z`)))
      (`NiagaraComponent.SetVariableVec3` (`self.Nia_Spark001_00`) "Beam End02" (`KismetMathLibrary.MakeVector` (`self.Spawn_Location_X`) (`self.Spawn_Location_Y`) (`self.Spawn_Location_Z`)))
      (`NiagaraComponent.SetVariableVec3` (`self.Nia_Spark001_00`) "Beam End03" (`KismetMathLibrary.MakeVector` (`self.Spawn_Location_X`) (`self.Spawn_Location_Y`) (`self.Spawn_Location_Z`)))
      (`NiagaraComponent.SetVariableVec3` (`self.Nia_Spark001_00`) "Beam Start01" (`KismetMathLibrary.MakeVector` (`self.Spawn_Location_X`) (`self.Spawn_Location_Y`)))
      (`NiagaraComponent.SetVariableVec3` (`self.Nia_Spark001_00`) "Beam Start02" (`KismetMathLibrary.MakeVector` (`self.Spawn_Location_X`) (`self.Spawn_Location_Y`)))
      (`NiagaraComponent.SetVariableVec3` (`self.Nia_Spark001_00`) "Beam Start03" (`KismetMathLibrary.MakeVector` (`self.Spawn_Location_X`) (`self.Spawn_Location_Y`))))
    (:`then_2`
      ;[1 1 1] 音
      (`GameplayStatics.PlaySound2D` "/Game/Player/sound/Cue/Cue_Thunder.Cue_Thunder" 1.0 1.0 0.0 null null))))

(fn `UserConstructionScript`)