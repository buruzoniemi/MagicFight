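; BP_iceBall is an ice ball actor under the player assets, with a Niagara component and a 2D ice sound played on BeginPlay.
; When it overlaps an actor tagged Land or Dragon, it spawns BP_iceDissolve at the Niagara component's location, intended as the damage area.
; The graph itself does not move the ball, apply damage or destroy it.
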(event `self.ReceiveActorBeginOverlap`
  (params (OtherActor :type "Actor Object Reference"))
  ;[1 1 1] 何かに当たったらダメージがある場所を用意する
  (`|ExecutionSequence`
    (:`then_0`
      (if (`self.ActorHasTag` OtherActor (`self.Land`))
        (`|SpawnActorFromClass` "/Game/Player/Actor/BP_iceDissolve.BP_iceDissolve_C" (`KismetMathLibrary.MakeTransform` (`SceneComponent.K2_GetComponentLocation` (`self.Niagara`))) "Undefined" "OverrideRootScale" null null :!label _label)))
    (:`then_1`
      (if (`self.ActorHasTag` OtherActor (`self.Dragon`))
        (goto _label)))))

(event `self.ReceiveBeginPlay`
  ;[1 1 1] 音
  (`GameplayStatics.PlaySound2D` "/Game/Player/sound/Cue/Cue_ice_2.Cue_ice_2" 1.0 1.0 0.0 null null))

(fn `UserConstructionScript`)