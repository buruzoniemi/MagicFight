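; BP_iceDissolve is a player-side ice effect actor that damages and slows dragons on overlap.
; When a Dragon-tagged actor overlaps, it moves to that actor's X/Y at a fixed height and starts a timeline that applies split damage through a delay on each update.
; In parallel, it lowers the walk speed of the Dragon_BP found by GetActorOfClass, rather than the overlapped actor, then restores it after a delay.
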(event `self.ReceiveActorBeginOverlap`
  (params (OtherActor :type "Actor Object Reference"))
  (bind (_returnvalue_x _returnvalue_y) (`KismetMathLibrary.BreakVector` (`self.K2_GetActorLocation` OtherActor)))
  ;[1 1 1] 当たった場所に展開する
  (`|ExecutionSequence`
    (:`then_0`
      (bind _returnvalue (`GameplayStatics.GetActorOfClass` "/Game/Enemy/Dorogon/Dragon_BP.Dragon_BP_C"))
      (set `self.Now_Location_X` _returnvalue_x)
      (set `self.Now_Location_Y` _returnvalue_y)
      (if (`self.ActorHasTag` OtherActor (`self.Dragon`))
        (`self.K2_SetActorTransform` (`KismetMathLibrary.MakeTransform` (`KismetMathLibrary.MakeVector` (`self.Now_Location_X`) (`self.Now_Location_Y`) 110.0)))
        ;[1 1 1] スプリットダメージのところ
        (`Timeline|タイムライン_0`
          (:`Update`
            (`KismetSystemLibrary.Delay` (`self.Sprit_Time`))
            (`GameplayStatics.ApplyDamage` OtherActor (`self.Ice_Sprit_Damage`))))))
    (:`then_2`
      ;[1 1 1] 当たった対象の移動速度を下げる
      (if (`self.ActorHasTag` OtherActor (`self.Dragon`))
        (bind _charactermovement (`Character.CharacterMovement` _returnvalue))
        (set `CharacterMovementComponent.MaxWalkSpeed` (`self.Walk_DownSpeed`) _charactermovement)
        (`KismetSystemLibrary.Delay` (`self.DownSpeed_Time`))
        (set `CharacterMovementComponent.MaxWalkSpeed` (`self.Reset_WalkSpeed`) _charactermovement)))))

(fn `UserConstructionScript`)