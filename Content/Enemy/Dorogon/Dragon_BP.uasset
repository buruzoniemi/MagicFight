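; Dragon boss enemy character with an HP bar, hit reactions and a death event that shows the game-clear widgets.
; Every fourth hit notifies Dragon_con and triggers knockback.
; Bite and claw events toggle head and hand overlap damage, while breath damage uses a timeline-driven fan of line traces.
; FallATK launches it airborne via timelines, spins the mesh, then explodes and damages the player regardless of distance.
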(event `self.ReceiveBeginPlay`
  ;[1 1 1] ゲームが始まったときの処理
  (`PrimitiveComponent.SetCollisionProfileName` (`self.Head`) "NoCollision" true)
  (`PrimitiveComponent.SetCollisionProfileName` (`self.RightHand`) "NoCollision" true)
  (bind _returnvalue (`|CreateWidget` "/Game/UI/BP/Chara_UI/BP_Enemy_HP_Bar.BP_Enemy_HP_Bar_C"))
  (bind _output_get (set `self.Enemy_HP_Bar` _returnvalue))
  (`UserWidget.AddToViewport` _output_get 0))

(event `FallATK`
  (params (NewParam :type Boolean))
  ;[1 1 1] HP変化による攻撃の変化（飛行）
  (set `self.StopBgm` true)
  (`|ExecutionSequence`
    (:`then_0`
      (`Timeline|タイムライン_0`
        (:`Update`
          (if (`NavMovementComponent.IsFalling` (`self.CharacterMovement`))
            (bind _asdragon_anim (cast `/Game/Enemy/Dorogon/DragonAnim` (`SkeletalMeshComponent.GetAnimInstance` (`self.Mesh`))))
            (set `/Game/Enemy/Dorogon/DragonAnim.It is Fry` true _asdragon_anim)
            (else
              (`|ExecutionSequence`
                (:`then_0`
                  (if (not (`self.DragonRotationStop`))
                    (bind _output_get (set `self.Delta Rotation` (`KismetMathLibrary.MakeRotator` (`self.FallAttackRotate`))))
                    (`SceneComponent.K2_AddLocalRotation` (`self.Mesh`) _output_get false false)
                    (set `self.ReFallAttackRotate` (+ (`self.FallAttackRotate`) (`self.ReFallAttackRotate`)))))
                (:`then_1`
                  (if (`self.FallAttackOnce`)
                    (set `self.FallAttackOnce` false)
                    (`KismetSystemLibrary.Delay` 5.0)
                    (`|PlayMontage` (`self.Mesh`) "/Game/Enemy/Dorogon/animmontage/Dragon_anim_mon_FallAttack.Dragon_anim_mon_FallAttack"
                      (:`then`
                        (set `self.DragonRotationStop` true))
                      (:`OnCompleted`
                        (bind _asdragon_anim_2 (cast `/Game/Enemy/Dorogon/DragonAnim` (`SkeletalMeshComponent.GetAnimInstance` (`self.Mesh`))))
                        (`KismetSystemLibrary.Delay` 0.5)
                        (`GameplayStatics.SpawnEmitterAtLocation` "/Game/MilitaryWeapDark/FX/P_Grenade_Explosion_01.P_Grenade_Explosion_01" (+ (`self.K2_GetActorLocation`) (0.0 0.0 -1500.0)) (struct) (100.0 100.0 100.0))
                        (`GameplayStatics.ApplyDamage` (`GameplayStatics.GetPlayerPawn` 0) 50.0)
                        (`KismetSystemLibrary.Delay` 2.6)
                        (set `/Game/Enemy/Dorogon/DragonAnim.It is Fry` false _asdragon_anim_2)
                        (bind _output_get_2 (set `self.ReFallAttackRotate` (* (`self.ReFallAttackRotate`) -1.0)))
                        (bind _output_get_3 (set `self.Delta Rotation` (`KismetMathLibrary.MakeRotator` _output_get_2)))
                        (`SceneComponent.K2_AddLocalRotation` (`self.Mesh`) _output_get_3 false false)
                        (set `self.StopBgm` false)))))))))))
    (:`then_1`
      (`Timeline|タイムライン_1`
        (:`Update`
          (`self.LaunchCharacter` (`self.Fry Velocity`)))
        (:`Finished`
          (`Timeline|タイムライン_2`
            (:`Update`
              (`self.LaunchCharacter` (`self.Fry Velocity2`)))))))))

(event `self.ReceiveAnyDamage`
  (params (Damage :type "Float (single-precision)") (DamageType :type "DamageType Object Reference") (InstigatedBy :type "Controller Object Reference") (DamageCauser :type "Actor Object Reference"))
  ;[1 1 1] ダメージを受けた時のアニメーション
  (`|ExecutionSequence`
    (:`then_0`
      (bind _output_get (set `self.HitCount` (+ (`self.HitCount`) 1.0)))
      (if (== _output_get 4.0)
        (bind _returnvalue (`GameplayStatics.GetActorOfClass` "/Game/Enemy/Dorogon/Dragon_con.Dragon_con_C"))
        (`/Game/Enemy/Dorogon/Dragon_con.Hit` _returnvalue)
        (set `self.HitCount` 0.0)
        (`KismetSystemLibrary.Delay` 0.05)
        (`self.Hit_Anim`)))
    (:`then_1`
      ;[1 1 1] ダメージ判定（判定が入ったらActorを消している）
      (bind _output_get_2 (set `self.HP` (- (`self.HP`) Damage)))
      (`/Game/UI/BP/Chara_UI/BP_Enemy_HP_Bar.Test1` (`self.Enemy_HP_Bar`) (/ _output_get_2 (`self.MaxHealth`))))))

(event `self.Head.OnComponentBeginOverlap`
  (params (OverlappedComponent :type "PrimitiveComponent Object Reference") (OtherActor :type "Actor Object Reference") (OtherComp :type "PrimitiveComponent Object Reference") (OtherBodyIndex :type Integer) (bFromSweep :type Boolean) (SweepResult :type "HitResult Structure (by ref)"))
  ;[1 1 1] 攻撃のダメージ
  (`/Engine/EditorBlueprintResources/StandardMacros.DoOnce` false :!label _label
    (:`Completed`
      (`GameplayStatics.ApplyDamage` OtherActor 5.0 null (`ActorComponent.GetOwner` (`self.Head`)))
      (`KismetSystemLibrary.Delay` 1.0)
      (goto _label :!via `Reset`))))

(event `self.RightHand.OnComponentBeginOverlap`
  (params (OverlappedComponent :type "PrimitiveComponent Object Reference") (OtherActor :type "Actor Object Reference") (OtherComp :type "PrimitiveComponent Object Reference") (OtherBodyIndex :type Integer) (bFromSweep :type Boolean) (SweepResult :type "HitResult Structure (by ref)"))
  ;[1 1 1] 攻撃のダメージ
  (`/Engine/EditorBlueprintResources/StandardMacros.DoOnce` false :!label _label_2
    (:`Completed`
      (`GameplayStatics.ApplyDamage` OtherActor 5.0 null (`ActorComponent.GetOwner` (`self.RightHand`)))
      (`KismetSystemLibrary.Delay` 1.0)
      (goto _label_2 :!via `Reset`))))

(event `Hit_Anim`
  ;[1 1 1] ノックバックのモーション
  (`self.LaunchCharacter` (1500.0 0.0 0.0))
  (`|PlayMontage` (`self.Mesh`) "/Game/Enemy/Dorogon/animmontage/Dragon_Anim_Mon_Hit.Dragon_Anim_Mon_Hit"))

(event `collisionActive_Bite`
  ;[1 1 1] Bite(噛みつきのタイミング)
  (`PrimitiveComponent.SetCollisionProfileName` (`self.Head`) "OverlapAll" true))

(event `collisionActive_Ripper`
  ;[1 1 1] Ripper(引き裂きのタイミング)
  (`PrimitiveComponent.SetCollisionProfileName` (`self.RightHand`) "OverlapAll" true))

(event `die`
  ;[1 1 1] 死んだ時のモーション
  (bind _asdragon_anim (cast `/Game/Enemy/Dorogon/DragonAnim` (`SkeletalMeshComponent.GetAnimInstance` (`self.Mesh`))))
  (set `/Game/Enemy/Dorogon/DragonAnim.die?` true _asdragon_anim)
  (`GameplayStatics.PlaySound2D` null 1.0 1.0 0.0 null null)
  (`|ExecutionSequence`
    (:`then_0`
      (bind _returnvalue (`|CreateWidget` "/Game/UI/BP/GameClear/BP_GameClear_Wall.BP_GameClear_Wall_C"))
      (`UserWidget.AddToViewport` _returnvalue 0))
    (:`then_1`
      (bind _returnvalue_2 (`|CreateWidget` "/Game/UI/BP/GameClear/BP_GameClear.BP_GameClear_C"))
      (`UserWidget.AddToViewport` _returnvalue_2 0)))
  (`KismetSystemLibrary.Delay` 3.0)
  (set `/Game/Enemy/Dorogon/DragonAnim.dienow?` true _asdragon_anim))

(event `collisionDeActive_Bite`
  ;[1 1 1] Bite(噛みつきのタイミング)
  (`PrimitiveComponent.SetCollisionProfileName` (`self.Head`) "NoCollision" true))

(event `collisionReActive_Ripper`
  ;[1 1 1] Ripper(引き裂きのタイミング)
  (`PrimitiveComponent.SetCollisionProfileName` (`self.RightHand`) "NoCollision" true))

(event `BlessOn`
  (bind _last_index (`self.Last Index`))
  (bind _returnvalue (+ (`self.K2_GetActorLocation`) (-450.0 0.0 -150.0)))
  ;[1 1 1] レイキャストによるブレスの辺り判定
  (`Timeline|ドラゴンのブレスの長さ` :!label _label_3
    (:`Update`
      (for _index (range (+ _last_index 1))
        (bind _outhit (`KismetSystemLibrary.LineTraceSingle` :`Start` _returnvalue :`End` (+ _returnvalue (* (`KismetMathLibrary.GreaterGreater_VectorRotator` (`self.GetActorRightVector`) (`KismetMathLibrary.MakeRotator` 0.0 0.0 (`KismetMathLibrary.Conv_IntToDouble` (* _index (/ 180 (+ _last_index 1)) -1)))) 800)) :`TraceChannel` "TraceTypeQuery1" :`DrawDebugType` "ForDuration"))
        (`GameplayStatics.ApplyDamage` (`.HitActor` (`GameplayStatics.BreakHitResult` _outhit)) 0.5)))))

(event `BlessOff`
  ;[1 1 1] レイキャストによるブレスの辺り判定
  (goto _label_3 :!via `Stop`))

(fn `UserConstructionScript`)